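; Mortar tower Blueprint that animates a track material and a hatch on its Tower mesh.
; ChangeSpeed zeroes the material's scroll speed, uses a timeline to lerp Speed into an Offset parameter, then restores scrolling from the final value.
; BeginPlay creates the dynamic track material and runs a timed demo of speed changes, with debug printing.
; ToggleHatch plays the open-hatch animation, though both FlipFlop branches set reverse playback.
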(event `self.ReceiveBeginPlay`
  (bind _returnvalue (`PrimitiveComponent.CreateDynamicMaterialInstance` (`self.Tower`) 1 "/Game/Towers/Mortar1/Tracks/M_Mortar1_Tracks.M_Mortar1_Tracks"))
  (set `self.Track Material` _returnvalue)
  (`MaterialInstanceDynamic.SetScalarParameterValue` (`self.Track Material`) "Speed X" (`self.Speed`))
  (`KismetSystemLibrary.Delay` 1.0)
  (`self.Change Speed` 1.0)
  (`KismetSystemLibrary.Delay` 3.0)
  (`self.Change Speed` 2.0)
  (`KismetSystemLibrary.Delay` 3.0)
  (`self.Change Speed` 0.0))

(event `Change Speed`
  (params (`New Speed` :type "Float (double-precision)"))
  (`MaterialInstanceDynamic.SetScalarParameterValue` (`self.Track Material`) "Speed X" 0.0)
  (set `self.New Speed` `New Speed`)
  (set `self.Old Speed` (`self.Speed`))
  (bind (_direction _alpha) (`Timeline|Change Speed Easing` :!via `PlayFromStart`)
    (:`Update`
      (`self.Set Offset` (`self.Old Speed`) (`self.New Speed`) _alpha))
    (:`Finished`
      (`MaterialInstanceDynamic.SetScalarParameterValue` (`self.Track Material`) "Speed X" (/ (`self.Speed`) 10.0)))))

(event `Toggle Hatch`
  (bind _tower (`self.Tower`))
  (`/Engine/EditorBlueprintResources/StandardMacros.FlipFlop`
    (:`A`
      (`SkeletalMeshComponent.SetPlayRate` _tower -1.0))
    (:`B`
      (`SkeletalMeshComponent.SetPlayRate` _tower -1.0)))
  (`SkeletalMeshComponent.PlayAnimation` _tower "/Game/Towers/Mortar1/Anim_Mortar_1_OpenHatch.Anim_Mortar_1_OpenHatch" false))

(fn `Set Offset`
  (params (`Old Speed` :type "Float (double-precision)") (`New SPeed` :type "Float (double-precision)") (Alpha :type "Float (double-precision)"))
  (bind _returnvalue (`KismetMathLibrary.Lerp` `Old Speed` `New SPeed` Alpha))
  (bind _output_get (set `self.Speed` _returnvalue))
  (`MeshComponent.SetScalarParameterValueOnMaterials` (`self.Tower`) "Offset" (/ _output_get 15.0))
  (`KismetSystemLibrary.PrintString` (`KismetStringLibrary.Conv_DoubleToString` _returnvalue)))

(fn `UserConstructionScript`
  (`parent.UserConstructionScript`))